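; BP_FuckingDrone is a drone actor that continuously turns to face a target pawn.
; On BeginPlay it stores the first entry from a search for all Pawn actors as its target, with no filter for player control.
; Every Tick it snaps its rotation toward that pawn with a look-at rotation, without interpolation or any movement logic.
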(event EventBeginPlay
  (bind _outactors (Actor|GetAllActorsOfClass "/Script/Engine.Pawn"))
  (if (Utilities|Array|IsValidIndex _outactors)
    (Variables|Default|SetTargetPawn (Utilities|Array|Get(acopy) _outactors))))

(event Collision|EventActorBeginOverlap
  (params (OtherActor :type Actor%20Object%20Reference)))

(event EventTick
  (params (DeltaSeconds :type Float%20%28single-precision%29))
  (Transformation|SetActorRotation (Math|Rotator|FindLookatRotation (Transformation|GetActorLocation) (Transformation|GetActorLocation (Variables|Default|GetTargetPawn)))))

(fn ConstructionScript)